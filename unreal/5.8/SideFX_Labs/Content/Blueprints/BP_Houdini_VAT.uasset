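; Houdini vertex animation texture (VAT) actor with controllable playback, optionally playing only while the player pawn overlaps its trigger box.
; The construction script applies a template mesh and material; initialization creates dynamic materials and calls an empty InitializeMode hook.
; Play, pause, reset, seek and rate functions store elapsed time, resume timestamp and rate.
; These values reach the materials as scalar parameters, so playback needs no Tick.
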(event `self.ReceiveBeginPlay`
  (`self.InitializeVAT`)
  (`KismetSystemLibrary.DelayUntilNextTick`)
  (`self.UpdateOverlapState`))

(event `self.OverlapTrigger.OnComponentBeginOverlap`
  (params (OverlappedComponent :type "PrimitiveComponent Object Reference") (OtherActor :type "Actor Object Reference") (OtherComp :type "PrimitiveComponent Object Reference") (OtherBodyIndex :type Integer) (bFromSweep :type Boolean) (SweepResult :type "HitResult Structure (by ref)"))
  (if (== OtherActor (`GameplayStatics.GetPlayerPawn` 0))
    (`self.UpdateOverlapState`)))

(event `self.OverlapTrigger.OnComponentEndOverlap`
  (params (OverlappedComponent :type "PrimitiveComponent Object Reference") (OtherActor :type "Actor Object Reference") (OtherComp :type "PrimitiveComponent Object Reference") (OtherBodyIndex :type Integer))
  (if (== OtherActor (`GameplayStatics.GetPlayerPawn` 0))
    (`self.UpdateOverlapState`)))

(fn `ApplyPlaybackState`
  (bind _vatmesh (`self.VATMesh`))
  (`MeshComponent.SetScalarParameterValueOnMaterials` _vatmesh "Use Playback Controls" 1.0)
  (`MeshComponent.SetScalarParameterValueOnMaterials` _vatmesh "Game Time at First Frame" 0.0)
  (`MeshComponent.SetScalarParameterValueOnMaterials` _vatmesh "VAT Playback Elapsed Time" (`self.PlaybackElapsed`))
  (`MeshComponent.SetScalarParameterValueOnMaterials` _vatmesh "VAT Playback Resume Time" (`self.PlaybackResumeTime`))
  (`MeshComponent.SetScalarParameterValueOnMaterials` _vatmesh "VAT Playback Rate" (`self.PlaybackRate`))
  (if (`self.PlaybackRunning`)
    (`MeshComponent.SetScalarParameterValueOnMaterials` _vatmesh "VAT Playback Running" 1.0)
    (`MeshComponent.SetScalarParameterValueOnMaterials` _vatmesh "Playback Speed" (`self.PlaybackRate`))
    (else
      (`MeshComponent.SetScalarParameterValueOnMaterials` _vatmesh "VAT Playback Running" 0.0)
      (`MeshComponent.SetScalarParameterValueOnMaterials` _vatmesh "Playback Speed" 0.0))))

(fn `CapturePlaybackTime`
  (if (`self.PlaybackRunning`)
    (set `self.PlaybackElapsed` (+ (`self.PlaybackElapsed`) (* (- (`KismetSystemLibrary.GetGameTimeInSeconds`) (`self.PlaybackResumeTime`)) (`self.PlaybackRate`))))
    (set `self.PlaybackResumeTime` (`KismetSystemLibrary.GetGameTimeInSeconds`))))

(fn `InitializeMode`)

(fn `InitializeVAT`
  (bind _overlaptrigger (`self.OverlapTrigger`))
  (bind _vatmesh (`self.VATMesh`))
  (if (not (`self.Initialized`))
    (`PrimitiveComponent.SetCollisionEnabled` _overlaptrigger "QueryOnly")
    (`PrimitiveComponent.SetCollisionResponseToAllChannels` _overlaptrigger "ECR_Ignore")
    (`PrimitiveComponent.SetCollisionResponseToChannel` _overlaptrigger "ECC_Pawn" "ECR_Overlap")
    (set `PrimitiveComponent.bGenerateOverlapEvents` true _overlaptrigger)
    (for _index (range (+ (- (`PrimitiveComponent.GetNumMaterials` (`self.VATMesh`)) 1) 1))
      (bind _returnvalue (`PrimitiveComponent.CreateDynamicMaterialInstance` _vatmesh _index (`PrimitiveComponent.GetMaterial` _vatmesh _index) "None"))
      (`/Engine/EditorBlueprintResources/StandardMacros.IsValid` _returnvalue
        (:`Is Valid`
          (`KismetArrayLibrary.Array_Add` (`self.DynamicMaterials`) _returnvalue))))
    (set `self.Initialized` true)
    (set `self.PlaybackRunning` false)
    (set `self.PlaybackElapsed` 0.0)
    (set `self.PlaybackResumeTime` 0.0)
    (`self.InitializeMode`)
    (`self.ApplyPlaybackState`)))

(fn `PauseVAT`
  (`self.InitializeVAT`)
  (`self.CapturePlaybackTime`)
  (set `self.PlaybackRunning` false)
  (`self.ApplyPlaybackState`))

(fn `PlayVAT`
  (`self.InitializeVAT`)
  (if (not (`self.PlaybackRunning`))
    (set `self.PlaybackResumeTime` (`KismetSystemLibrary.GetGameTimeInSeconds`))
    (set `self.PlaybackRunning` true)
    (`self.ApplyPlaybackState`)))

(fn `ResetVAT`
  (`self.InitializeVAT`)
  (set `self.PlaybackElapsed` 0.0)
  (set `self.PlaybackResumeTime` (`KismetSystemLibrary.GetGameTimeInSeconds`))
  (set `self.PlaybackRunning` false)
  (`self.ApplyPlaybackState`))

(fn `RestartVAT`
  (`self.ResetVAT`)
  (`self.PlayVAT`))

(fn `ResumeVAT`
  (`self.PlayVAT`))

(fn `SeekVAT`
  (params (TimeSeconds :type "Float (double-precision)"))
  (if (and (>= TimeSeconds 0.0) (== (- TimeSeconds TimeSeconds) 0.0))
    (`self.InitializeVAT`)
    (set `self.PlaybackElapsed` TimeSeconds)
    (set `self.PlaybackResumeTime` (`KismetSystemLibrary.GetGameTimeInSeconds`))
    (`self.ApplyPlaybackState`)))

(fn `SetVATPlaybackRate`
  (params (Rate :type "Float (double-precision)"))
  (if (and (>= Rate 0.0) (== (- Rate Rate) 0.0))
    (`self.InitializeVAT`)
    (`self.CapturePlaybackTime`)
    (set `self.PlaybackRate` Rate)
    (set `self.PlaybackResumeTime` (`KismetSystemLibrary.GetGameTimeInSeconds`))
    (`self.ApplyPlaybackState`)))

(fn `UpdateOverlapState`
  (bind _returnvalue (`GameplayStatics.GetPlayerPawn` 0))
  (if (`self.UsePlayerOverlap`)
    (`/Engine/EditorBlueprintResources/StandardMacros.IsValid` _returnvalue
      (:`Is Valid`
        (if (`PrimitiveComponent.IsOverlappingActor` (`self.OverlapTrigger`) _returnvalue)
          (`self.ResumeVAT`)
          (else
            (`self.PauseVAT`))))
      (:`Is Not Valid`
        (`self.PauseVAT`)))))

(fn `UserConstructionScript`
  (bind _vatmesh (`self.VATMesh`))
  (bind _templatemesh (`self.TemplateMesh`))
  (bind _templatematerial (`self.TemplateMaterial`))
  (`/Engine/EditorBlueprintResources/StandardMacros.IsValid` _templatemesh
    (:`Is Valid`
      (`StaticMeshComponent.SetStaticMesh` _vatmesh _templatemesh)
      (`/Engine/EditorBlueprintResources/StandardMacros.IsValid` _templatematerial
        (:`Is Valid`
          (for _index (range (+ (- (`PrimitiveComponent.GetNumMaterials` _vatmesh) 1) 1))
            (`PrimitiveComponent.SetMaterial` _vatmesh _index _templatematerial)
            (`BoxComponent.SetBoxExtent` (`self.OverlapTrigger`) (`self.In Box Extent`) true)))))))