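; PCG Blueprint node that imports Houdini-exported points from two DataTables, CSVMesh and CSVData.
; Execution joins mesh or actor and material paths into comma-separated strings, then iterates per CSVMesh row.
; Each point swaps Y/Z, rebuilds quaternion W, applies per-mesh and global transforms, and takes density and color from CSVData.
; Unless DeleteAttributes is set, row indices select mesh and material attributes, written alongside IDs and custom floats.
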(fn ExecutewithContext
  (params (InContext :type PCG%20Context%20Structure%20%28by%20ref%29) (Input :type PCG%20Data%20Collection%20Structure%20%28by%20ref%29))
  (Utilities|FlowControl|Sequence
    (:then_0
      (if (Variables|ActorReferences|GetSwitchToActors)
        ;[1 1 1] Actors
        (for _array_element (Variables|ActorReferences|GetActors)
          (Variables|Default|SetMeshPaths (Utilities|String|Append (Variables|Default|GetMeshPaths) (Utilities|String|Append _array_element ",")))
          (Variables|Default|SetActor%20Count (+ (Variables|Default|GetActor%20Count) 1)))
        (else
          (Utilities|FlowControl|Sequence
            (:then_0
              ;[0.5579 0.5906 1] Loop over all the Mesh Entries and Append them into one large string where the meshes are seperated by a comma
              (for _array_element_2 (Variables|ConfigFiles|GetMeshes)
                (Variables|Default|SetMeshPaths (Utilities|String|Append (Variables|Default|GetMeshPaths) (Utilities|String|Append (Utilities|ToString(SoftObjectReference) _array_element_2) ",")))
                (Variables|Default|SetMesh%20Count (+ (Variables|Default|GetMesh%20Count) 1))))
            (:then_1
              ;[0.5579 0.5906 1] Loop over all the Material Entries and Append them into one large string where the meshes are seperated by a comma
              (for _array_element_3 (Variables|MaterialOverrides|GetMaterial)
                (Variables|Default|SetMaterialPaths (Utilities|String|Append (Variables|Default|GetMaterialPaths) (Utilities|String|Append (Utilities|ToString(SoftObjectReference) _array_element_3) ",")))
                (Variables|Default|SetMaterial%20Count (+ (Variables|Default|GetMaterial%20Count) 1))))
            (:then_2
              ;[0.5579 0.5906 1] Loop over all the Material Entries and Append them into one large string where the meshes are seperated by a comma
              (for _array_element_4 (Variables|MaterialOverrides|GetMaterial_1)
                (Variables|Default|SetMaterial_1_Paths (Utilities|String|Append (Variables|Default|GetMaterial_1_Paths) (Utilities|String|Append (Utilities|ToString(SoftObjectReference) _array_element_4) ",")))
                (Variables|Default|SetMaterial_1_Count (+ (Variables|Default|GetMaterial_1_Count) 1))))
            (:then_3
              ;[0.5579 0.5906 1] Loop over all the Material Entries and Append them into one large string where the meshes are seperated by a comma
              (for _array_element_5 (Variables|MaterialOverrides|GetMaterial_2)
                (Variables|Default|SetMaterial_2_Paths (Utilities|String|Append (Variables|Default|GetMaterial_2_Paths) (Utilities|String|Append (Utilities|ToString(SoftObjectReference) _array_element_5) ",")))
                (Variables|Default|SetMaterial_2_Count (+ (Variables|Default|GetMaterial_2_Count) 1))))
            (:then_4
              ;[0.5579 0.5906 1] Loop over all the Material Entries and Append them into one large string where the meshes are seperated by a comma
              (for _array_element_6 (Variables|MaterialOverrides|GetMaterial_3)
                (Variables|Default|SetMaterial_3_Paths (Utilities|String|Append (Variables|Default|GetMaterial_3_Paths) (Utilities|String|Append (Utilities|ToString(SoftObjectReference) _array_element_6) ",")))
                (Variables|Default|SetMaterial_3_Count (+ (Variables|Default|GetMaterial_3_Count) 1))))
            (:then_5
              ;[0.5579 0.5906 1] Loop over all the Material Entries and Append them into one large string where the meshes are seperated by a comma
              (for _array_element_7 (Variables|MaterialOverrides|GetMaterial_4)
                (Variables|Default|SetMaterial_4_Paths (Utilities|String|Append (Variables|Default|GetMaterial_4_Paths) (Utilities|String|Append (Utilities|ToString(SoftObjectReference) _array_element_7) ",")))
                (Variables|Default|SetMaterial_4_Count (+ (Variables|Default|GetMaterial_4_Count) 1))))
            (:then_6
              ;[0.5579 0.5906 1] Loop over all the Material Entries and Append them into one large string where the meshes are seperated by a comma
              (for _array_element_8 (Variables|MaterialOverrides|GetMaterial_5)
                (Variables|Default|SetMaterial_5_Paths (Utilities|String|Append (Variables|Default|GetMaterial_5_Paths) (Utilities|String|Append (Utilities|ToString(SoftObjectReference) _array_element_8) ",")))
                (Variables|Default|SetMaterial_5_Count (+ (Variables|Default|GetMaterial_5_Count) 1))))))))
    (:then_1
      (Utilities|FlowControl|Sequence
        (:then_0
          ;[0.5579 0.5906 1] Get number of points from CSV file
          (bind _outrownames (DataTable|GetDataTableRowNames (Variables|ConfigFiles|GetCSV%20Mesh)))
          (for _array_element_9 _outrownames
            (bind _returnvalue (Utilities|GetDataTableRow (Variables|ConfigFiles|GetCSV%20Mesh) _array_element_9)
              (:then
                (Variables|Default|SetNumberOfPoints (+ 1 (Variables|Default|GetNumberOfPoints)))))))
        (:then_1
          ;[0.5579 0.5906 1] Get number of points from CSV file
          (bind _outrownames_2 (DataTable|GetDataTableRowNames (Variables|ConfigFiles|GetCSV%20Data)))
          (for _array_element_10 _outrownames_2
            (bind _returnvalue_2 (Utilities|GetDataTableRow (Variables|ConfigFiles|GetCSV%20Data) _array_element_10)
              (:then
                (Variables|Default|SetNumberOfPoints_Data (+ 1 (Variables|Default|GetNumberOfPoints_Data))))))
          (Variables|Default|SetMatchingDataTables (== (Variables|Default|GetNumberOfPoints) (Variables|Default|GetNumberOfPoints_Data))))))
    (:then_2
      (bind _output_get (LocalVariables|SetInputCollection Input))
      (Class|PCGDataFunctionLibrary|GetInputs _output_get)
      (bind _output_get_2 (LocalVariables|SetContext InContext))
      (bind _returnvalue_3 (PCG|Temporary|GetActorData _output_get_2))
      ;[1 1 1] Make PCG iteration loop
      (bind _aspcgspatial_data (Utilities|Casting|CastToPCGSpatialData _returnvalue_3))
      (Variables|Default|SetContext%20PCGSpatial%20Data _aspcgspatial_data)
      (Utilities|Array|Clear (LocalVariables|GetOutPoints))
      (bind _outdata (PCG|FlowControl|IterationLoop (LocalVariables|GetContext) (Class|KismetMathLibrary|ToInt64(Integer) (Variables|Default|GetNumberOfPoints)) 0 0 0))
      (return (Utilities|Struct|MakePCGDataCollection (Utilities|Array|MakeArray (Utilities|Struct|MakePCGTaggedData _outdata 0 "None")))))))

(fn NodeTitleOverride
  (return "Houdini Import Data Table"))

(fn IterationLoopBody
  (params (InContext :type PCG%20Context%20Structure%20%28by%20ref%29) (Iteration :type Integer64) (InA :type PCG%20Spatial%20Data%20Object%20Reference) (InB :type PCG%20Spatial%20Data%20Object%20Reference) (OutMetadata :type PCG%20Metadata%20Object%20Reference))
  (bind _material_2_paths (Variables|Default|GetMaterial_2_Paths))
  (bind _material_1_paths (Variables|Default|GetMaterial_1_Paths))
  (bind _expand_points (Variables|ExtraTransforms|GetExpand%20Points))
  (bind _meshpaths (Variables|Default|GetMeshPaths))
  (bind _material_3_paths (Variables|Default|GetMaterial_3_Paths))
  (bind _materialpaths (Variables|Default|GetMaterialPaths))
  (bind _global_transform (Variables|ExtraTransforms|GetGlobal%20Transform))
  (bind _material_4_paths (Variables|Default|GetMaterial_4_Paths))
  (bind _material_5_paths (Variables|Default|GetMaterial_5_Paths))
  (bind _returnvalue (Utilities|String|ParseIntoArray _meshpaths ","))
  (bind _returnvalue_2 (Utilities|String|ParseIntoArray _material_2_paths ","))
  (bind _returnvalue_3 (Utilities|String|ParseIntoArray _material_3_paths ","))
  (bind _returnvalue_4 (Utilities|String|ParseIntoArray _material_4_paths ","))
  (bind (_location _rotation _scale) (Math|Transform|BreakTransform _global_transform))
  (bind _returnvalue_5 (Utilities|String|ParseIntoArray _materialpaths ","))
  (bind _returnvalue_6 (Utilities|String|ParseIntoArray _material_1_paths ","))
  (bind _returnvalue_7 (Utilities|String|ParseIntoArray _material_5_paths ","))
  (LocalVariables|SetMetaData OutMetadata)
  (LocalVariables|SetIter Iteration)
  (if (Variables|ConfigFiles|GetDelete%20Attributes)
    _
    (else
      ;[1 1 1] Initialize Mesh Attribute
      (PCG|Metadata|CreateStringAttribute (LocalVariables|GetMetaData) "mesh" (Utilities|Array|Get(acopy) _returnvalue) false true)
      ;[1 1 1] Initialize MeshType, Mesh and Material Attributes as Floats
      (PCG|Metadata|CreateFloatAttribute (LocalVariables|GetMetaData) "mesh_id" 0.0 false true)
      (PCG|Metadata|CreateFloatAttribute (LocalVariables|GetMetaData) "material_id" 0.0 false true)
      (PCG|Metadata|CreateFloatAttribute (LocalVariables|GetMetaData) "material_1_id" 0.0 false true)
      (PCG|Metadata|CreateFloatAttribute (LocalVariables|GetMetaData) "material_2_id" 0.0 false true)
      (PCG|Metadata|CreateFloatAttribute (LocalVariables|GetMetaData) "material_3_id" 0.0 false true)
      (PCG|Metadata|CreateFloatAttribute (LocalVariables|GetMetaData) "material_4_id" 0.0 false true)
      (PCG|Metadata|CreateFloatAttribute (LocalVariables|GetMetaData) "material_5_id" 0.0 false true)
      (PCG|Metadata|CreateFloatAttribute (LocalVariables|GetMetaData) "custom_float" 0.0 false true)
      (PCG|Metadata|CreateFloatAttribute (LocalVariables|GetMetaData) "custom_float_1" 0.0 false true)
      (PCG|Metadata|CreateFloatAttribute (LocalVariables|GetMetaData) "custom_float_2" 0.0 false true)
      (PCG|Metadata|CreateFloatAttribute (LocalVariables|GetMetaData) "custom_float_3" 0.0 false true)))
  ;[1 1 1] Run a loop over CSV Rows (Check if the two CSVs are matching, if not, only use the first)
  (bind _outrownames (DataTable|GetDataTableRowNames (Variables|ConfigFiles|GetCSV%20Mesh)))
  (bind _returnvalue_8 (Utilities|GetDataTableRow (Variables|ConfigFiles|GetCSV%20Mesh) (Utilities|Array|Get(acopy) _outrownames (Math|Conversions|ToInteger(Byte) (LocalVariables|GetIter))))
    (:then
      (bind _returnvalue_9 (Utilities|GetDataTableRow (Variables|ConfigFiles|GetCSV%20Data) (Utilities|Array|Get(acopy) _outrownames (Math|Conversions|ToInteger(Byte) (LocalVariables|GetIter))))
        (:then
          (if (Variables|ConfigFiles|GetDelete%20Attributes)
            _
            (else
              ;[1 1 1] Apply Material
              (PCG|Metadata|CreateStringAttribute (LocalVariables|GetMetaData) "material" (Utilities|Array|Get(acopy) _returnvalue_5) false true)
              (PCG|Metadata|CreateStringAttribute (LocalVariables|GetMetaData) "material_1" (Utilities|Array|Get(acopy) _returnvalue_6) false true)
              (PCG|Metadata|CreateStringAttribute (LocalVariables|GetMetaData) "material_2" (Utilities|Array|Get(acopy) _returnvalue_2) false true)
              (PCG|Metadata|CreateStringAttribute (LocalVariables|GetMetaData) "material_3" (Utilities|Array|Get(acopy) _returnvalue_3) false true)
              (PCG|Metadata|CreateStringAttribute (LocalVariables|GetMetaData) "material_4" (Utilities|Array|Get(acopy) _returnvalue_4) false true)
              (PCG|Metadata|CreateStringAttribute (LocalVariables|GetMetaData) "material_5" (Utilities|Array|Get(acopy) _returnvalue_7) false true)
              (Class|PCGMetadataAccessorHelpers|SetStringAttribute (Utilities|Struct|MakePCGPoint (Math|Transform|MakeTransform (+ (* (Math|Vector|MakeVector _expand_points _expand_points _expand_points) (Math|Vector|MakeVector (.Px (Utilities|Struct|BreakCSVPointFormat _returnvalue_8)) (.Pz (Utilities|Struct|BreakCSVPointFormat _returnvalue_8)) (.Py (Utilities|Struct|BreakCSVPointFormat _returnvalue_8)))) (+ (.Location (Math|Transform|BreakTransform (Utilities|Array|Get(acopy) (Variables|ExtraTransforms|GetPer%20Mesh%20Transforms) (Math|Float|Truncate (.pscale (Utilities|Struct|BreakCSVPointFormat _returnvalue_8)))))) _location)) (Math|Rotator|CombineRotators (Class|KismetMathLibrary|QuatRotator (Class|KismetMathLibrary|MakeQuat (.Nx (Utilities|Struct|BreakCSVPointFormat _returnvalue_8)) (.Nz (Utilities|Struct|BreakCSVPointFormat _returnvalue_8)) (.Ny (Utilities|Struct|BreakCSVPointFormat _returnvalue_8)) (* (Math|Float|Sqrt (- (- (- (Math|Float|MakeLiteralFloat 1.0) (* (.Nx (Utilities|Struct|BreakCSVPointFormat _returnvalue_8)) (.Nx (Utilities|Struct|BreakCSVPointFormat _returnvalue_8)))) (* (.Ny (Utilities|Struct|BreakCSVPointFormat _returnvalue_8)) (.Ny (Utilities|Struct|BreakCSVPointFormat _returnvalue_8)))) (* (.Nz (Utilities|Struct|BreakCSVPointFormat _returnvalue_8)) (.Nz (Utilities|Struct|BreakCSVPointFormat _returnvalue_8))))) -1.0))) (Math|Rotator|CombineRotators (.Rotation (Math|Transform|BreakTransform (Utilities|Array|Get(acopy) (Variables|ExtraTransforms|GetPer%20Mesh%20Transforms) (Math|Float|Truncate (.pscale (Utilities|Struct|BreakCSVPointFormat _returnvalue_8)))))) _rotation)) (* (Math|Vector|MakeVector (.UVx (Utilities|Struct|BreakCSVPointFormat _returnvalue_8)) (.UVz (Utilities|Struct|BreakCSVPointFormat _returnvalue_8)) (.UVy (Utilities|Struct|BreakCSVPointFormat _returnvalue_8))) (* (.Scale (Math|Transform|BreakTransform (Utilities|Array|Get(acopy) (Variables|ExtraTransforms|GetPer%20Mesh%20Transforms) (Math|Float|Truncate (.pscale (Utilities|Struct|BreakCSVPointFormat _returnvalue_8)))))) _scale))) (.pscale (Utilities|Struct|BreakCSVPointFormat _returnvalue_9)) (Math|Vector4|MakeVector4 (.UVx (Utilities|Struct|BreakCSVPointFormat _returnvalue_9)) (.UVy (Utilities|Struct|BreakCSVPointFormat _returnvalue_9)) (.UVz (Utilities|Struct|BreakCSVPointFormat _returnvalue_9)) 1.0)) (LocalVariables|GetMetaData) "material" (Utilities|Array|Get(acopy) _returnvalue_5 (Math|Float|Truncate (.Px (Utilities|Struct|BreakCSVPointFormat _returnvalue_9)))))
              (Class|PCGMetadataAccessorHelpers|SetStringAttribute (Utilities|Struct|MakePCGPoint (Math|Transform|MakeTransform (+ (* (Math|Vector|MakeVector _expand_points _expand_points _expand_points) (Math|Vector|MakeVector (.Px (Utilities|Struct|BreakCSVPointFormat _returnvalue_8)) (.Pz (Utilities|Struct|BreakCSVPointFormat _returnvalue_8)) (.Py (Utilities|Struct|BreakCSVPointFormat _returnvalue_8)))) (+ (.Location (Math|Transform|BreakTransform (Utilities|Array|Get(acopy) (Variables|ExtraTransforms|GetPer%20Mesh%20Transforms) (Math|Float|Truncate (.pscale (Utilities|Struct|BreakCSVPointFormat _returnvalue_8)))))) _location)) (Math|Rotator|CombineRotators (Class|KismetMathLibrary|QuatRotator (Class|KismetMathLibrary|MakeQuat (.Nx (Utilities|Struct|BreakCSVPointFormat _returnvalue_8)) (.Nz (Utilities|Struct|BreakCSVPointFormat _returnvalue_8)) (.Ny (Utilities|Struct|BreakCSVPointFormat _returnvalue_8)) (* (Math|Float|Sqrt (- (- (- (Math|Float|MakeLiteralFloat 1.0) (* (.Nx (Utilities|Struct|BreakCSVPointFormat _returnvalue_8)) (.Nx (Utilities|Struct|BreakCSVPointFormat _returnvalue_8)))) (* (.Ny (Utilities|Struct|BreakCSVPointFormat _returnvalue_8)) (.Ny (Utilities|Struct|BreakCSVPointFormat _returnvalue_8)))) (* (.Nz (Utilities|Struct|BreakCSVPointFormat _returnvalue_8)) (.Nz (Utilities|Struct|BreakCSVPointFormat _returnvalue_8))))) -1.0))) (Math|Rotator|CombineRotators (.Rotation (Math|Transform|BreakTransform (Utilities|Array|Get(acopy) (Variables|ExtraTransforms|GetPer%20Mesh%20Transforms) (Math|Float|Truncate (.pscale (Utilities|Struct|BreakCSVPointFormat _returnvalue_8)))))) _rotation)) (* (Math|Vector|MakeVector (.UVx (Utilities|Struct|BreakCSVPointFormat _returnvalue_8)) (.UVz (Utilities|Struct|BreakCSVPointFormat _returnvalue_8)) (.UVy (Utilities|Struct|BreakCSVPointFormat _returnvalue_8))) (* (.Scale (Math|Transform|BreakTransform (Utilities|Array|Get(acopy) (Variables|ExtraTransforms|GetPer%20Mesh%20Transforms) (Math|Float|Truncate (.pscale (Utilities|Struct|BreakCSVPointFormat _returnvalue_8)))))) _scale))) (.pscale (Utilities|Struct|BreakCSVPointFormat _returnvalue_9)) (Math|Vector4|MakeVector4 (.UVx (Utilities|Struct|BreakCSVPointFormat _returnvalue_9)) (.UVy (Utilities|Struct|BreakCSVPointFormat _returnvalue_9)) (.UVz (Utilities|Struct|BreakCSVPointFormat _returnvalue_9)) 1.0)) (LocalVariables|GetMetaData) "material_1" (Utilities|Array|Get(acopy) _returnvalue_6 (Math|Float|Truncate (.Py (Utilities|Struct|BreakCSVPointFormat _returnvalue_9)))))
              (Class|PCGMetadataAccessorHelpers|SetStringAttribute (Utilities|Struct|MakePCGPoint (Math|Transform|MakeTransform (+ (* (Math|Vector|MakeVector _expand_points _expand_points _expand_points) (Math|Vector|MakeVector (.Px (Utilities|Struct|BreakCSVPointFormat _returnvalue_8)) (.Pz (Utilities|Struct|BreakCSVPointFormat _returnvalue_8)) (.Py (Utilities|Struct|BreakCSVPointFormat _returnvalue_8)))) (+ (.Location (Math|Transform|BreakTransform (Utilities|Array|Get(acopy) (Variables|ExtraTransforms|GetPer%20Mesh%20Transforms) (Math|Float|Truncate (.pscale (Utilities|Struct|BreakCSVPointFormat _returnvalue_8)))))) _location)) (Math|Rotator|CombineRotators (Class|KismetMathLibrary|QuatRotator (Class|KismetMathLibrary|MakeQuat (.Nx (Utilities|Struct|BreakCSVPointFormat _returnvalue_8)) (.Nz (Utilities|Struct|BreakCSVPointFormat _returnvalue_8)) (.Ny (Utilities|Struct|BreakCSVPointFormat _returnvalue_8)) (* (Math|Float|Sqrt (- (- (- (Math|Float|MakeLiteralFloat 1.0) (* (.Nx (Utilities|Struct|BreakCSVPointFormat _returnvalue_8)) (.Nx (Utilities|Struct|BreakCSVPointFormat _returnvalue_8)))) (* (.Ny (Utilities|Struct|BreakCSVPointFormat _returnvalue_8)) (.Ny (Utilities|Struct|BreakCSVPointFormat _returnvalue_8)))) (* (.Nz (Utilities|Struct|BreakCSVPointFormat _returnvalue_8)) (.Nz (Utilities|Struct|BreakCSVPointFormat _returnvalue_8))))) -1.0))) (Math|Rotator|CombineRotators (.Rotation (Math|Transform|BreakTransform (Utilities|Array|Get(acopy) (Variables|ExtraTransforms|GetPer%20Mesh%20Transforms) (Math|Float|Truncate (.pscale (Utilities|Struct|BreakCSVPointFormat _returnvalue_8)))))) _rotation)) (* (Math|Vector|MakeVector (.UVx (Utilities|Struct|BreakCSVPointFormat _returnvalue_8)) (.UVz (Utilities|Struct|BreakCSVPointFormat _returnvalue_8)) (.UVy (Utilities|Struct|BreakCSVPointFormat _returnvalue_8))) (* (.Scale (Math|Transform|BreakTransform (Utilities|Array|Get(acopy) (Variables|ExtraTransforms|GetPer%20Mesh%20Transforms) (Math|Float|Truncate (.pscale (Utilities|Struct|BreakCSVPointFormat _returnvalue_8)))))) _scale))) (.pscale (Utilities|Struct|BreakCSVPointFormat _returnvalue_9)) (Math|Vector4|MakeVector4 (.UVx (Utilities|Struct|BreakCSVPointFormat _returnvalue_9)) (.UVy (Utilities|Struct|BreakCSVPointFormat _returnvalue_9)) (.UVz (Utilities|Struct|BreakCSVPointFormat _returnvalue_9)) 1.0)) (LocalVariables|GetMetaData) "material_2" (Utilities|Array|Get(acopy) _returnvalue_2 (Math|Float|Truncate (.Pz (Utilities|Struct|BreakCSVPointFormat _returnvalue_9)))))
              (Class|PCGMetadataAccessorHelpers|SetStringAttribute (Utilities|Struct|MakePCGPoint (Math|Transform|MakeTransform (+ (* (Math|Vector|MakeVector _expand_points _expand_points _expand_points) (Math|Vector|MakeVector (.Px (Utilities|Struct|BreakCSVPointFormat _returnvalue_8)) (.Pz (Utilities|Struct|BreakCSVPointFormat _returnvalue_8)) (.Py (Utilities|Struct|BreakCSVPointFormat _returnvalue_8)))) (+ (.Location (Math|Transform|BreakTransform (Utilities|Array|Get(acopy) (Variables|ExtraTransforms|GetPer%20Mesh%20Transforms) (Math|Float|Truncate (.pscale (Utilities|Struct|BreakCSVPointFormat _returnvalue_8)))))) _location)) (Math|Rotator|CombineRotators (Class|KismetMathLibrary|QuatRotator (Class|KismetMathLibrary|MakeQuat (.Nx (Utilities|Struct|BreakCSVPointFormat _returnvalue_8)) (.Nz (Utilities|Struct|BreakCSVPointFormat _returnvalue_8)) (.Ny (Utilities|Struct|BreakCSVPointFormat _returnvalue_8)) (* (Math|Float|Sqrt (- (- (- (Math|Float|MakeLiteralFloat 1.0) (* (.Nx (Utilities|Struct|BreakCSVPointFormat _returnvalue_8)) (.Nx (Utilities|Struct|BreakCSVPointFormat _returnvalue_8)))) (* (.Ny (Utilities|Struct|BreakCSVPointFormat _returnvalue_8)) (.Ny (Utilities|Struct|BreakCSVPointFormat _returnvalue_8)))) (* (.Nz (Utilities|Struct|BreakCSVPointFormat _returnvalue_8)) (.Nz (Utilities|Struct|BreakCSVPointFormat _returnvalue_8))))) -1.0))) (Math|Rotator|CombineRotators (.Rotation (Math|Transform|BreakTransform (Utilities|Array|Get(acopy) (Variables|ExtraTransforms|GetPer%20Mesh%20Transforms) (Math|Float|Truncate (.pscale (Utilities|Struct|BreakCSVPointFormat _returnvalue_8)))))) _rotation)) (* (Math|Vector|MakeVector (.UVx (Utilities|Struct|BreakCSVPointFormat _returnvalue_8)) (.UVz (Utilities|Struct|BreakCSVPointFormat _returnvalue_8)) (.UVy (Utilities|Struct|BreakCSVPointFormat _returnvalue_8))) (* (.Scale (Math|Transform|BreakTransform (Utilities|Array|Get(acopy) (Variables|ExtraTransforms|GetPer%20Mesh%20Transforms) (Math|Float|Truncate (.pscale (Utilities|Struct|BreakCSVPointFormat _returnvalue_8)))))) _scale))) (.pscale (Utilities|Struct|BreakCSVPointFormat _returnvalue_9)) (Math|Vector4|MakeVector4 (.UVx (Utilities|Struct|BreakCSVPointFormat _returnvalue_9)) (.UVy (Utilities|Struct|BreakCSVPointFormat _returnvalue_9)) (.UVz (Utilities|Struct|BreakCSVPointFormat _returnvalue_9)) 1.0)) (LocalVariables|GetMetaData) "material_3" (Utilities|Array|Get(acopy) _returnvalue_3 (Math|Float|Truncate (.Nx (Utilities|Struct|BreakCSVPointFormat _returnvalue_9)))))
              (Class|PCGMetadataAccessorHelpers|SetStringAttribute (Utilities|Struct|MakePCGPoint (Math|Transform|MakeTransform (+ (* (Math|Vector|MakeVector _expand_points _expand_points _expand_points) (Math|Vector|MakeVector (.Px (Utilities|Struct|BreakCSVPointFormat _returnvalue_8)) (.Pz (Utilities|Struct|BreakCSVPointFormat _returnvalue_8)) (.Py (Utilities|Struct|BreakCSVPointFormat _returnvalue_8)))) (+ (.Location (Math|Transform|BreakTransform (Utilities|Array|Get(acopy) (Variables|ExtraTransforms|GetPer%20Mesh%20Transforms) (Math|Float|Truncate (.pscale (Utilities|Struct|BreakCSVPointFormat _returnvalue_8)))))) _location)) (Math|Rotator|CombineRotators (Class|KismetMathLibrary|QuatRotator (Class|KismetMathLibrary|MakeQuat (.Nx (Utilities|Struct|BreakCSVPointFormat _returnvalue_8)) (.Nz (Utilities|Struct|BreakCSVPointFormat _returnvalue_8)) (.Ny (Utilities|Struct|BreakCSVPointFormat _returnvalue_8)) (* (Math|Float|Sqrt (- (- (- (Math|Float|MakeLiteralFloat 1.0) (* (.Nx (Utilities|Struct|BreakCSVPointFormat _returnvalue_8)) (.Nx (Utilities|Struct|BreakCSVPointFormat _returnvalue_8)))) (* (.Ny (Utilities|Struct|BreakCSVPointFormat _returnvalue_8)) (.Ny (Utilities|Struct|BreakCSVPointFormat _returnvalue_8)))) (* (.Nz (Utilities|Struct|BreakCSVPointFormat _returnvalue_8)) (.Nz (Utilities|Struct|BreakCSVPointFormat _returnvalue_8))))) -1.0))) (Math|Rotator|CombineRotators (.Rotation (Math|Transform|BreakTransform (Utilities|Array|Get(acopy) (Variables|ExtraTransforms|GetPer%20Mesh%20Transforms) (Math|Float|Truncate (.pscale (Utilities|Struct|BreakCSVPointFormat _returnvalue_8)))))) _rotation)) (* (Math|Vector|MakeVector (.UVx (Utilities|Struct|BreakCSVPointFormat _returnvalue_8)) (.UVz (Utilities|Struct|BreakCSVPointFormat _returnvalue_8)) (.UVy (Utilities|Struct|BreakCSVPointFormat _returnvalue_8))) (* (.Scale (Math|Transform|BreakTransform (Utilities|Array|Get(acopy) (Variables|ExtraTransforms|GetPer%20Mesh%20Transforms) (Math|Float|Truncate (.pscale (Utilities|Struct|BreakCSVPointFormat _returnvalue_8)))))) _scale))) (.pscale (Utilities|Struct|BreakCSVPointFormat _returnvalue_9)) (Math|Vector4|MakeVector4 (.UVx (Utilities|Struct|BreakCSVPointFormat _returnvalue_9)) (.UVy (Utilities|Struct|BreakCSVPointFormat _returnvalue_9)) (.UVz (Utilities|Struct|BreakCSVPointFormat _returnvalue_9)) 1.0)) (LocalVariables|GetMetaData) "material_4" (Utilities|Array|Get(acopy) _returnvalue_4 (Math|Float|Truncate (.Ny (Utilities|Struct|BreakCSVPointFormat _returnvalue_9)))))
              (Class|PCGMetadataAccessorHelpers|SetStringAttribute (Utilities|Struct|MakePCGPoint (Math|Transform|MakeTransform (+ (* (Math|Vector|MakeVector _expand_points _expand_points _expand_points) (Math|Vector|MakeVector (.Px (Utilities|Struct|BreakCSVPointFormat _returnvalue_8)) (.Pz (Utilities|Struct|BreakCSVPointFormat _returnvalue_8)) (.Py (Utilities|Struct|BreakCSVPointFormat _returnvalue_8)))) (+ (.Location (Math|Transform|BreakTransform (Utilities|Array|Get(acopy) (Variables|ExtraTransforms|GetPer%20Mesh%20Transforms) (Math|Float|Truncate (.pscale (Utilities|Struct|BreakCSVPointFormat _returnvalue_8)))))) _location)) (Math|Rotator|CombineRotators (Class|KismetMathLibrary|QuatRotator (Class|KismetMathLibrary|MakeQuat (.Nx (Utilities|Struct|BreakCSVPointFormat _returnvalue_8)) (.Nz (Utilities|Struct|BreakCSVPointFormat _returnvalue_8)) (.Ny (Utilities|Struct|BreakCSVPointFormat _returnvalue_8)) (* (Math|Float|Sqrt (- (- (- (Math|Float|MakeLiteralFloat 1.0) (* (.Nx (Utilities|Struct|BreakCSVPointFormat _returnvalue_8)) (.Nx (Utilities|Struct|BreakCSVPointFormat _returnvalue_8)))) (* (.Ny (Utilities|Struct|BreakCSVPointFormat _returnvalue_8)) (.Ny (Utilities|Struct|BreakCSVPointFormat _returnvalue_8)))) (* (.Nz (Utilities|Struct|BreakCSVPointFormat _returnvalue_8)) (.Nz (Utilities|Struct|BreakCSVPointFormat _returnvalue_8))))) -1.0))) (Math|Rotator|CombineRotators (.Rotation (Math|Transform|BreakTransform (Utilities|Array|Get(acopy) (Variables|ExtraTransforms|GetPer%20Mesh%20Transforms) (Math|Float|Truncate (.pscale (Utilities|Struct|BreakCSVPointFormat _returnvalue_8)))))) _rotation)) (* (Math|Vector|MakeVector (.UVx (Utilities|Struct|BreakCSVPointFormat _returnvalue_8)) (.UVz (Utilities|Struct|BreakCSVPointFormat _returnvalue_8)) (.UVy (Utilities|Struct|BreakCSVPointFormat _returnvalue_8))) (* (.Scale (Math|Transform|BreakTransform (Utilities|Array|Get(acopy) (Variables|ExtraTransforms|GetPer%20Mesh%20Transforms) (Math|Float|Truncate (.pscale (Utilities|Struct|BreakCSVPointFormat _returnvalue_8)))))) _scale))) (.pscale (Utilities|Struct|BreakCSVPointFormat _returnvalue_9)) (Math|Vector4|MakeVector4 (.UVx (Utilities|Struct|BreakCSVPointFormat _returnvalue_9)) (.UVy (Utilities|Struct|BreakCSVPointFormat _returnvalue_9)) (.UVz (Utilities|Struct|BreakCSVPointFormat _returnvalue_9)) 1.0)) (LocalVariables|GetMetaData) "material_5" (Utilities|Array|Get(acopy) _returnvalue_7 (Math|Float|Truncate (.Nz (Utilities|Struct|BreakCSVPointFormat _returnvalue_9)))))
              ;[1 1 1] Set Mesh and MeshType Float Values
              (PCG|Metadata|SetFloatAttribute (Utilities|Struct|MakePCGPoint (Math|Transform|MakeTransform (+ (* (Math|Vector|MakeVector _expand_points _expand_points _expand_points) (Math|Vector|MakeVector (.Px (Utilities|Struct|BreakCSVPointFormat _returnvalue_8)) (.Pz (Utilities|Struct|BreakCSVPointFormat _returnvalue_8)) (.Py (Utilities|Struct|BreakCSVPointFormat _returnvalue_8)))) (+ (.Location (Math|Transform|BreakTransform (Utilities|Array|Get(acopy) (Variables|ExtraTransforms|GetPer%20Mesh%20Transforms) (Math|Float|Truncate (.pscale (Utilities|Struct|BreakCSVPointFormat _returnvalue_8)))))) _location)) (Math|Rotator|CombineRotators (Class|KismetMathLibrary|QuatRotator (Class|KismetMathLibrary|MakeQuat (.Nx (Utilities|Struct|BreakCSVPointFormat _returnvalue_8)) (.Nz (Utilities|Struct|BreakCSVPointFormat _returnvalue_8)) (.Ny (Utilities|Struct|BreakCSVPointFormat _returnvalue_8)) (* (Math|Float|Sqrt (- (- (- (Math|Float|MakeLiteralFloat 1.0) (* (.Nx (Utilities|Struct|BreakCSVPointFormat _returnvalue_8)) (.Nx (Utilities|Struct|BreakCSVPointFormat _returnvalue_8)))) (* (.Ny (Utilities|Struct|BreakCSVPointFormat _returnvalue_8)) (.Ny (Utilities|Struct|BreakCSVPointFormat _returnvalue_8)))) (* (.Nz (Utilities|Struct|BreakCSVPointFormat _returnvalue_8)) (.Nz (Utilities|Struct|BreakCSVPointFormat _returnvalue_8))))) -1.0))) (Math|Rotator|CombineRotators (.Rotation (Math|Transform|BreakTransform (Utilities|Array|Get(acopy) (Variables|ExtraTransforms|GetPer%20Mesh%20Transforms) (Math|Float|Truncate (.pscale (Utilities|Struct|BreakCSVPointFormat _returnvalue_8)))))) _rotation)) (* (Math|Vector|MakeVector (.UVx (Utilities|Struct|BreakCSVPointFormat _returnvalue_8)) (.UVz (Utilities|Struct|BreakCSVPointFormat _returnvalue_8)) (.UVy (Utilities|Struct|BreakCSVPointFormat _returnvalue_8))) (* (.Scale (Math|Transform|BreakTransform (Utilities|Array|Get(acopy) (Variables|ExtraTransforms|GetPer%20Mesh%20Transforms) (Math|Float|Truncate (.pscale (Utilities|Struct|BreakCSVPointFormat _returnvalue_8)))))) _scale))) (.pscale (Utilities|Struct|BreakCSVPointFormat _returnvalue_9)) (Math|Vector4|MakeVector4 (.UVx (Utilities|Struct|BreakCSVPointFormat _returnvalue_9)) (.UVy (Utilities|Struct|BreakCSVPointFormat _returnvalue_9)) (.UVz (Utilities|Struct|BreakCSVPointFormat _returnvalue_9)) 1.0)) (LocalVariables|GetMetaData) "mesh_id" (.pscale (Utilities|Struct|BreakCSVPointFormat _returnvalue_8)))
              (PCG|Metadata|SetFloatAttribute (Utilities|Struct|MakePCGPoint (Math|Transform|MakeTransform (+ (* (Math|Vector|MakeVector _expand_points _expand_points _expand_points) (Math|Vector|MakeVector (.Px (Utilities|Struct|BreakCSVPointFormat _returnvalue_8)) (.Pz (Utilities|Struct|BreakCSVPointFormat _returnvalue_8)) (.Py (Utilities|Struct|BreakCSVPointFormat _returnvalue_8)))) (+ (.Location (Math|Transform|BreakTransform (Utilities|Array|Get(acopy) (Variables|ExtraTransforms|GetPer%20Mesh%20Transforms) (Math|Float|Truncate (.pscale (Utilities|Struct|BreakCSVPointFormat _returnvalue_8)))))) _location)) (Math|Rotator|CombineRotators (Class|KismetMathLibrary|QuatRotator (Class|KismetMathLibrary|MakeQuat (.Nx (Utilities|Struct|BreakCSVPointFormat _returnvalue_8)) (.Nz (Utilities|Struct|BreakCSVPointFormat _returnvalue_8)) (.Ny (Utilities|Struct|BreakCSVPointFormat _returnvalue_8)) (* (Math|Float|Sqrt (- (- (- (Math|Float|MakeLiteralFloat 1.0) (* (.Nx (Utilities|Struct|BreakCSVPointFormat _returnvalue_8)) (.Nx (Utilities|Struct|BreakCSVPointFormat _returnvalue_8)))) (* (.Ny (Utilities|Struct|BreakCSVPointFormat _returnvalue_8)) (.Ny (Utilities|Struct|BreakCSVPointFormat _returnvalue_8)))) (* (.Nz (Utilities|Struct|BreakCSVPointFormat _returnvalue_8)) (.Nz (Utilities|Struct|BreakCSVPointFormat _returnvalue_8))))) -1.0))) (Math|Rotator|CombineRotators (.Rotation (Math|Transform|BreakTransform (Utilities|Array|Get(acopy) (Variables|ExtraTransforms|GetPer%20Mesh%20Transforms) (Math|Float|Truncate (.pscale (Utilities|Struct|BreakCSVPointFormat _returnvalue_8)))))) _rotation)) (* (Math|Vector|MakeVector (.UVx (Utilities|Struct|BreakCSVPointFormat _returnvalue_8)) (.UVz (Utilities|Struct|BreakCSVPointFormat _returnvalue_8)) (.UVy (Utilities|Struct|BreakCSVPointFormat _returnvalue_8))) (* (.Scale (Math|Transform|BreakTransform (Utilities|Array|Get(acopy) (Variables|ExtraTransforms|GetPer%20Mesh%20Transforms) (Math|Float|Truncate (.pscale (Utilities|Struct|BreakCSVPointFormat _returnvalue_8)))))) _scale))) (.pscale (Utilities|Struct|BreakCSVPointFormat _returnvalue_9)) (Math|Vector4|MakeVector4 (.UVx (Utilities|Struct|BreakCSVPointFormat _returnvalue_9)) (.UVy (Utilities|Struct|BreakCSVPointFormat _returnvalue_9)) (.UVz (Utilities|Struct|BreakCSVPointFormat _returnvalue_9)) 1.0)) (LocalVariables|GetMetaData) "material_id" (.Px (Utilities|Struct|BreakCSVPointFormat _returnvalue_9)))
              (PCG|Metadata|SetFloatAttribute (Utilities|Struct|MakePCGPoint (Math|Transform|MakeTransform (+ (* (Math|Vector|MakeVector _expand_points _expand_points _expand_points) (Math|Vector|MakeVector (.Px (Utilities|Struct|BreakCSVPointFormat _returnvalue_8)) (.Pz (Utilities|Struct|BreakCSVPointFormat _returnvalue_8)) (.Py (Utilities|Struct|BreakCSVPointFormat _returnvalue_8)))) (+ (.Location (Math|Transform|BreakTransform (Utilities|Array|Get(acopy) (Variables|ExtraTransforms|GetPer%20Mesh%20Transforms) (Math|Float|Truncate (.pscale (Utilities|Struct|BreakCSVPointFormat _returnvalue_8)))))) _location)) (Math|Rotator|CombineRotators (Class|KismetMathLibrary|QuatRotator (Class|KismetMathLibrary|MakeQuat (.Nx (Utilities|Struct|BreakCSVPointFormat _returnvalue_8)) (.Nz (Utilities|Struct|BreakCSVPointFormat _returnvalue_8)) (.Ny (Utilities|Struct|BreakCSVPointFormat _returnvalue_8)) (* (Math|Float|Sqrt (- (- (- (Math|Float|MakeLiteralFloat 1.0) (* (.Nx (Utilities|Struct|BreakCSVPointFormat _returnvalue_8)) (.Nx (Utilities|Struct|BreakCSVPointFormat _returnvalue_8)))) (* (.Ny (Utilities|Struct|BreakCSVPointFormat _returnvalue_8)) (.Ny (Utilities|Struct|BreakCSVPointFormat _returnvalue_8)))) (* (.Nz (Utilities|Struct|BreakCSVPointFormat _returnvalue_8)) (.Nz (Utilities|Struct|BreakCSVPointFormat _returnvalue_8))))) -1.0))) (Math|Rotator|CombineRotators (.Rotation (Math|Transform|BreakTransform (Utilities|Array|Get(acopy) (Variables|ExtraTransforms|GetPer%20Mesh%20Transforms) (Math|Float|Truncate (.pscale (Utilities|Struct|BreakCSVPointFormat _returnvalue_8)))))) _rotation)) (* (Math|Vector|MakeVector (.UVx (Utilities|Struct|BreakCSVPointFormat _returnvalue_8)) (.UVz (Utilities|Struct|BreakCSVPointFormat _returnvalue_8)) (.UVy (Utilities|Struct|BreakCSVPointFormat _returnvalue_8))) (* (.Scale (Math|Transform|BreakTransform (Utilities|Array|Get(acopy) (Variables|ExtraTransforms|GetPer%20Mesh%20Transforms) (Math|Float|Truncate (.pscale (Utilities|Struct|BreakCSVPointFormat _returnvalue_8)))))) _scale))) (.pscale (Utilities|Struct|BreakCSVPointFormat _returnvalue_9)) (Math|Vector4|MakeVector4 (.UVx (Utilities|Struct|BreakCSVPointFormat _returnvalue_9)) (.UVy (Utilities|Struct|BreakCSVPointFormat _returnvalue_9)) (.UVz (Utilities|Struct|BreakCSVPointFormat _returnvalue_9)) 1.0)) (LocalVariables|GetMetaData) "material_1_id" (.Py (Utilities|Struct|BreakCSVPointFormat _returnvalue_9)))
              (PCG|Metadata|SetFloatAttribute (Utilities|Struct|MakePCGPoint (Math|Transform|MakeTransform (+ (* (Math|Vector|MakeVector _expand_points _expand_points _expand_points) (Math|Vector|MakeVector (.Px (Utilities|Struct|BreakCSVPointFormat _returnvalue_8)) (.Pz (Utilities|Struct|BreakCSVPointFormat _returnvalue_8)) (.Py (Utilities|Struct|BreakCSVPointFormat _returnvalue_8)))) (+ (.Location (Math|Transform|BreakTransform (Utilities|Array|Get(acopy) (Variables|ExtraTransforms|GetPer%20Mesh%20Transforms) (Math|Float|Truncate (.pscale (Utilities|Struct|BreakCSVPointFormat _returnvalue_8)))))) _location)) (Math|Rotator|CombineRotators (Class|KismetMathLibrary|QuatRotator (Class|KismetMathLibrary|MakeQuat (.Nx (Utilities|Struct|BreakCSVPointFormat _returnvalue_8)) (.Nz (Utilities|Struct|BreakCSVPointFormat _returnvalue_8)) (.Ny (Utilities|Struct|BreakCSVPointFormat _returnvalue_8)) (* (Math|Float|Sqrt (- (- (- (Math|Float|MakeLiteralFloat 1.0) (* (.Nx (Utilities|Struct|BreakCSVPointFormat _returnvalue_8)) (.Nx (Utilities|Struct|BreakCSVPointFormat _returnvalue_8)))) (* (.Ny (Utilities|Struct|BreakCSVPointFormat _returnvalue_8)) (.Ny (Utilities|Struct|BreakCSVPointFormat _returnvalue_8)))) (* (.Nz (Utilities|Struct|BreakCSVPointFormat _returnvalue_8)) (.Nz (Utilities|Struct|BreakCSVPointFormat _returnvalue_8))))) -1.0))) (Math|Rotator|CombineRotators (.Rotation (Math|Transform|BreakTransform (Utilities|Array|Get(acopy) (Variables|ExtraTransforms|GetPer%20Mesh%20Transforms) (Math|Float|Truncate (.pscale (Utilities|Struct|BreakCSVPointFormat _returnvalue_8)))))) _rotation)) (* (Math|Vector|MakeVector (.UVx (Utilities|Struct|BreakCSVPointFormat _returnvalue_8)) (.UVz (Utilities|Struct|BreakCSVPointFormat _returnvalue_8)) (.UVy (Utilities|Struct|BreakCSVPointFormat _returnvalue_8))) (* (.Scale (Math|Transform|BreakTransform (Utilities|Array|Get(acopy) (Variables|ExtraTransforms|GetPer%20Mesh%20Transforms) (Math|Float|Truncate (.pscale (Utilities|Struct|BreakCSVPointFormat _returnvalue_8)))))) _scale))) (.pscale (Utilities|Struct|BreakCSVPointFormat _returnvalue_9)) (Math|Vector4|MakeVector4 (.UVx (Utilities|Struct|BreakCSVPointFormat _returnvalue_9)) (.UVy (Utilities|Struct|BreakCSVPointFormat _returnvalue_9)) (.UVz (Utilities|Struct|BreakCSVPointFormat _returnvalue_9)) 1.0)) (LocalVariables|GetMetaData) "material_2_id" (.Pz (Utilities|Struct|BreakCSVPointFormat _returnvalue_9)))
              (PCG|Metadata|SetFloatAttribute (Utilities|Struct|MakePCGPoint (Math|Transform|MakeTransform (+ (* (Math|Vector|MakeVector _expand_points _expand_points _expand_points) (Math|Vector|MakeVector (.Px (Utilities|Struct|BreakCSVPointFormat _returnvalue_8)) (.Pz (Utilities|Struct|BreakCSVPointFormat _returnvalue_8)) (.Py (Utilities|Struct|BreakCSVPointFormat _returnvalue_8)))) (+ (.Location (Math|Transform|BreakTransform (Utilities|Array|Get(acopy) (Variables|ExtraTransforms|GetPer%20Mesh%20Transforms) (Math|Float|Truncate (.pscale (Utilities|Struct|BreakCSVPointFormat _returnvalue_8)))))) _location)) (Math|Rotator|CombineRotators (Class|KismetMathLibrary|QuatRotator (Class|KismetMathLibrary|MakeQuat (.Nx (Utilities|Struct|BreakCSVPointFormat _returnvalue_8)) (.Nz (Utilities|Struct|BreakCSVPointFormat _returnvalue_8)) (.Ny (Utilities|Struct|BreakCSVPointFormat _returnvalue_8)) (* (Math|Float|Sqrt (- (- (- (Math|Float|MakeLiteralFloat 1.0) (* (.Nx (Utilities|Struct|BreakCSVPointFormat _returnvalue_8)) (.Nx (Utilities|Struct|BreakCSVPointFormat _returnvalue_8)))) (* (.Ny (Utilities|Struct|BreakCSVPointFormat _returnvalue_8)) (.Ny (Utilities|Struct|BreakCSVPointFormat _returnvalue_8)))) (* (.Nz (Utilities|Struct|BreakCSVPointFormat _returnvalue_8)) (.Nz (Utilities|Struct|BreakCSVPointFormat _returnvalue_8))))) -1.0))) (Math|Rotator|CombineRotators (.Rotation (Math|Transform|BreakTransform (Utilities|Array|Get(acopy) (Variables|ExtraTransforms|GetPer%20Mesh%20Transforms) (Math|Float|Truncate (.pscale (Utilities|Struct|BreakCSVPointFormat _returnvalue_8)))))) _rotation)) (* (Math|Vector|MakeVector (.UVx (Utilities|Struct|BreakCSVPointFormat _returnvalue_8)) (.UVz (Utilities|Struct|BreakCSVPointFormat _returnvalue_8)) (.UVy (Utilities|Struct|BreakCSVPointFormat _returnvalue_8))) (* (.Scale (Math|Transform|BreakTransform (Utilities|Array|Get(acopy) (Variables|ExtraTransforms|GetPer%20Mesh%20Transforms) (Math|Float|Truncate (.pscale (Utilities|Struct|BreakCSVPointFormat _returnvalue_8)))))) _scale))) (.pscale (Utilities|Struct|BreakCSVPointFormat _returnvalue_9)) (Math|Vector4|MakeVector4 (.UVx (Utilities|Struct|BreakCSVPointFormat _returnvalue_9)) (.UVy (Utilities|Struct|BreakCSVPointFormat _returnvalue_9)) (.UVz (Utilities|Struct|BreakCSVPointFormat _returnvalue_9)) 1.0)) (LocalVariables|GetMetaData) "material_3_id" (.Nx (Utilities|Struct|BreakCSVPointFormat _returnvalue_9)))
              (PCG|Metadata|SetFloatAttribute (Utilities|Struct|MakePCGPoint (Math|Transform|MakeTransform (+ (* (Math|Vector|MakeVector _expand_points _expand_points _expand_points) (Math|Vector|MakeVector (.Px (Utilities|Struct|BreakCSVPointFormat _returnvalue_8)) (.Pz (Utilities|Struct|BreakCSVPointFormat _returnvalue_8)) (.Py (Utilities|Struct|BreakCSVPointFormat _returnvalue_8)))) (+ (.Location (Math|Transform|BreakTransform (Utilities|Array|Get(acopy) (Variables|ExtraTransforms|GetPer%20Mesh%20Transforms) (Math|Float|Truncate (.pscale (Utilities|Struct|BreakCSVPointFormat _returnvalue_8)))))) _location)) (Math|Rotator|CombineRotators (Class|KismetMathLibrary|QuatRotator (Class|KismetMathLibrary|MakeQuat (.Nx (Utilities|Struct|BreakCSVPointFormat _returnvalue_8)) (.Nz (Utilities|Struct|BreakCSVPointFormat _returnvalue_8)) (.Ny (Utilities|Struct|BreakCSVPointFormat _returnvalue_8)) (* (Math|Float|Sqrt (- (- (- (Math|Float|MakeLiteralFloat 1.0) (* (.Nx (Utilities|Struct|BreakCSVPointFormat _returnvalue_8)) (.Nx (Utilities|Struct|BreakCSVPointFormat _returnvalue_8)))) (* (.Ny (Utilities|Struct|BreakCSVPointFormat _returnvalue_8)) (.Ny (Utilities|Struct|BreakCSVPointFormat _returnvalue_8)))) (* (.Nz (Utilities|Struct|BreakCSVPointFormat _returnvalue_8)) (.Nz (Utilities|Struct|BreakCSVPointFormat _returnvalue_8))))) -1.0))) (Math|Rotator|CombineRotators (.Rotation (Math|Transform|BreakTransform (Utilities|Array|Get(acopy) (Variables|ExtraTransforms|GetPer%20Mesh%20Transforms) (Math|Float|Truncate (.pscale (Utilities|Struct|BreakCSVPointFormat _returnvalue_8)))))) _rotation)) (* (Math|Vector|MakeVector (.UVx (Utilities|Struct|BreakCSVPointFormat _returnvalue_8)) (.UVz (Utilities|Struct|BreakCSVPointFormat _returnvalue_8)) (.UVy (Utilities|Struct|BreakCSVPointFormat _returnvalue_8))) (* (.Scale (Math|Transform|BreakTransform (Utilities|Array|Get(acopy) (Variables|ExtraTransforms|GetPer%20Mesh%20Transforms) (Math|Float|Truncate (.pscale (Utilities|Struct|BreakCSVPointFormat _returnvalue_8)))))) _scale))) (.pscale (Utilities|Struct|BreakCSVPointFormat _returnvalue_9)) (Math|Vector4|MakeVector4 (.UVx (Utilities|Struct|BreakCSVPointFormat _returnvalue_9)) (.UVy (Utilities|Struct|BreakCSVPointFormat _returnvalue_9)) (.UVz (Utilities|Struct|BreakCSVPointFormat _returnvalue_9)) 1.0)) (LocalVariables|GetMetaData) "material_4_id" (.Ny (Utilities|Struct|BreakCSVPointFormat _returnvalue_9)))
              (PCG|Metadata|SetFloatAttribute (Utilities|Struct|MakePCGPoint (Math|Transform|MakeTransform (+ (* (Math|Vector|MakeVector _expand_points _expand_points _expand_points) (Math|Vector|MakeVector (.Px (Utilities|Struct|BreakCSVPointFormat _returnvalue_8)) (.Pz (Utilities|Struct|BreakCSVPointFormat _returnvalue_8)) (.Py (Utilities|Struct|BreakCSVPointFormat _returnvalue_8)))) (+ (.Location (Math|Transform|BreakTransform (Utilities|Array|Get(acopy) (Variables|ExtraTransforms|GetPer%20Mesh%20Transforms) (Math|Float|Truncate (.pscale (Utilities|Struct|BreakCSVPointFormat _returnvalue_8)))))) _location)) (Math|Rotator|CombineRotators (Class|KismetMathLibrary|QuatRotator (Class|KismetMathLibrary|MakeQuat (.Nx (Utilities|Struct|BreakCSVPointFormat _returnvalue_8)) (.Nz (Utilities|Struct|BreakCSVPointFormat _returnvalue_8)) (.Ny (Utilities|Struct|BreakCSVPointFormat _returnvalue_8)) (* (Math|Float|Sqrt (- (- (- (Math|Float|MakeLiteralFloat 1.0) (* (.Nx (Utilities|Struct|BreakCSVPointFormat _returnvalue_8)) (.Nx (Utilities|Struct|BreakCSVPointFormat _returnvalue_8)))) (* (.Ny (Utilities|Struct|BreakCSVPointFormat _returnvalue_8)) (.Ny (Utilities|Struct|BreakCSVPointFormat _returnvalue_8)))) (* (.Nz (Utilities|Struct|BreakCSVPointFormat _returnvalue_8)) (.Nz (Utilities|Struct|BreakCSVPointFormat _returnvalue_8))))) -1.0))) (Math|Rotator|CombineRotators (.Rotation (Math|Transform|BreakTransform (Utilities|Array|Get(acopy) (Variables|ExtraTransforms|GetPer%20Mesh%20Transforms) (Math|Float|Truncate (.pscale (Utilities|Struct|BreakCSVPointFormat _returnvalue_8)))))) _rotation)) (* (Math|Vector|MakeVector (.UVx (Utilities|Struct|BreakCSVPointFormat _returnvalue_8)) (.UVz (Utilities|Struct|BreakCSVPointFormat _returnvalue_8)) (.UVy (Utilities|Struct|BreakCSVPointFormat _returnvalue_8))) (* (.Scale (Math|Transform|BreakTransform (Utilities|Array|Get(acopy) (Variables|ExtraTransforms|GetPer%20Mesh%20Transforms) (Math|Float|Truncate (.pscale (Utilities|Struct|BreakCSVPointFormat _returnvalue_8)))))) _scale))) (.pscale (Utilities|Struct|BreakCSVPointFormat _returnvalue_9)) (Math|Vector4|MakeVector4 (.UVx (Utilities|Struct|BreakCSVPointFormat _returnvalue_9)) (.UVy (Utilities|Struct|BreakCSVPointFormat _returnvalue_9)) (.UVz (Utilities|Struct|BreakCSVPointFormat _returnvalue_9)) 1.0)) (LocalVariables|GetMetaData) "material_5_id" (.Nz (Utilities|Struct|BreakCSVPointFormat _returnvalue_9)))
              (PCG|Metadata|SetFloatAttribute (Utilities|Struct|MakePCGPoint (Math|Transform|MakeTransform (+ (* (Math|Vector|MakeVector _expand_points _expand_points _expand_points) (Math|Vector|MakeVector (.Px (Utilities|Struct|BreakCSVPointFormat _returnvalue_8)) (.Pz (Utilities|Struct|BreakCSVPointFormat _returnvalue_8)) (.Py (Utilities|Struct|BreakCSVPointFormat _returnvalue_8)))) (+ (.Location (Math|Transform|BreakTransform (Utilities|Array|Get(acopy) (Variables|ExtraTransforms|GetPer%20Mesh%20Transforms) (Math|Float|Truncate (.pscale (Utilities|Struct|BreakCSVPointFormat _returnvalue_8)))))) _location)) (Math|Rotator|CombineRotators (Class|KismetMathLibrary|QuatRotator (Class|KismetMathLibrary|MakeQuat (.Nx (Utilities|Struct|BreakCSVPointFormat _returnvalue_8)) (.Nz (Utilities|Struct|BreakCSVPointFormat _returnvalue_8)) (.Ny (Utilities|Struct|BreakCSVPointFormat _returnvalue_8)) (* (Math|Float|Sqrt (- (- (- (Math|Float|MakeLiteralFloat 1.0) (* (.Nx (Utilities|Struct|BreakCSVPointFormat _returnvalue_8)) (.Nx (Utilities|Struct|BreakCSVPointFormat _returnvalue_8)))) (* (.Ny (Utilities|Struct|BreakCSVPointFormat _returnvalue_8)) (.Ny (Utilities|Struct|BreakCSVPointFormat _returnvalue_8)))) (* (.Nz (Utilities|Struct|BreakCSVPointFormat _returnvalue_8)) (.Nz (Utilities|Struct|BreakCSVPointFormat _returnvalue_8))))) -1.0))) (Math|Rotator|CombineRotators (.Rotation (Math|Transform|BreakTransform (Utilities|Array|Get(acopy) (Variables|ExtraTransforms|GetPer%20Mesh%20Transforms) (Math|Float|Truncate (.pscale (Utilities|Struct|BreakCSVPointFormat _returnvalue_8)))))) _rotation)) (* (Math|Vector|MakeVector (.UVx (Utilities|Struct|BreakCSVPointFormat _returnvalue_8)) (.UVz (Utilities|Struct|BreakCSVPointFormat _returnvalue_8)) (.UVy (Utilities|Struct|BreakCSVPointFormat _returnvalue_8))) (* (.Scale (Math|Transform|BreakTransform (Utilities|Array|Get(acopy) (Variables|ExtraTransforms|GetPer%20Mesh%20Transforms) (Math|Float|Truncate (.pscale (Utilities|Struct|BreakCSVPointFormat _returnvalue_8)))))) _scale))) (.pscale (Utilities|Struct|BreakCSVPointFormat _returnvalue_9)) (Math|Vector4|MakeVector4 (.UVx (Utilities|Struct|BreakCSVPointFormat _returnvalue_9)) (.UVy (Utilities|Struct|BreakCSVPointFormat _returnvalue_9)) (.UVz (Utilities|Struct|BreakCSVPointFormat _returnvalue_9)) 1.0)) (LocalVariables|GetMetaData) "custom_float" (.UVx (Utilities|Struct|BreakCSVPointFormat _returnvalue_9)))
              (PCG|Metadata|SetFloatAttribute (Utilities|Struct|MakePCGPoint (Math|Transform|MakeTransform (+ (* (Math|Vector|MakeVector _expand_points _expand_points _expand_points) (Math|Vector|MakeVector (.Px (Utilities|Struct|BreakCSVPointFormat _returnvalue_8)) (.Pz (Utilities|Struct|BreakCSVPointFormat _returnvalue_8)) (.Py (Utilities|Struct|BreakCSVPointFormat _returnvalue_8)))) (+ (.Location (Math|Transform|BreakTransform (Utilities|Array|Get(acopy) (Variables|ExtraTransforms|GetPer%20Mesh%20Transforms) (Math|Float|Truncate (.pscale (Utilities|Struct|BreakCSVPointFormat _returnvalue_8)))))) _location)) (Math|Rotator|CombineRotators (Class|KismetMathLibrary|QuatRotator (Class|KismetMathLibrary|MakeQuat (.Nx (Utilities|Struct|BreakCSVPointFormat _returnvalue_8)) (.Nz (Utilities|Struct|BreakCSVPointFormat _returnvalue_8)) (.Ny (Utilities|Struct|BreakCSVPointFormat _returnvalue_8)) (* (Math|Float|Sqrt (- (- (- (Math|Float|MakeLiteralFloat 1.0) (* (.Nx (Utilities|Struct|BreakCSVPointFormat _returnvalue_8)) (.Nx (Utilities|Struct|BreakCSVPointFormat _returnvalue_8)))) (* (.Ny (Utilities|Struct|BreakCSVPointFormat _returnvalue_8)) (.Ny (Utilities|Struct|BreakCSVPointFormat _returnvalue_8)))) (* (.Nz (Utilities|Struct|BreakCSVPointFormat _returnvalue_8)) (.Nz (Utilities|Struct|BreakCSVPointFormat _returnvalue_8))))) -1.0))) (Math|Rotator|CombineRotators (.Rotation (Math|Transform|BreakTransform (Utilities|Array|Get(acopy) (Variables|ExtraTransforms|GetPer%20Mesh%20Transforms) (Math|Float|Truncate (.pscale (Utilities|Struct|BreakCSVPointFormat _returnvalue_8)))))) _rotation)) (* (Math|Vector|MakeVector (.UVx (Utilities|Struct|BreakCSVPointFormat _returnvalue_8)) (.UVz (Utilities|Struct|BreakCSVPointFormat _returnvalue_8)) (.UVy (Utilities|Struct|BreakCSVPointFormat _returnvalue_8))) (* (.Scale (Math|Transform|BreakTransform (Utilities|Array|Get(acopy) (Variables|ExtraTransforms|GetPer%20Mesh%20Transforms) (Math|Float|Truncate (.pscale (Utilities|Struct|BreakCSVPointFormat _returnvalue_8)))))) _scale))) (.pscale (Utilities|Struct|BreakCSVPointFormat _returnvalue_9)) (Math|Vector4|MakeVector4 (.UVx (Utilities|Struct|BreakCSVPointFormat _returnvalue_9)) (.UVy (Utilities|Struct|BreakCSVPointFormat _returnvalue_9)) (.UVz (Utilities|Struct|BreakCSVPointFormat _returnvalue_9)) 1.0)) (LocalVariables|GetMetaData) "custom_float_1" (.UVy (Utilities|Struct|BreakCSVPointFormat _returnvalue_9)))
              (PCG|Metadata|SetFloatAttribute (Utilities|Struct|MakePCGPoint (Math|Transform|MakeTransform (+ (* (Math|Vector|MakeVector _expand_points _expand_points _expand_points) (Math|Vector|MakeVector (.Px (Utilities|Struct|BreakCSVPointFormat _returnvalue_8)) (.Pz (Utilities|Struct|BreakCSVPointFormat _returnvalue_8)) (.Py (Utilities|Struct|BreakCSVPointFormat _returnvalue_8)))) (+ (.Location (Math|Transform|BreakTransform (Utilities|Array|Get(acopy) (Variables|ExtraTransforms|GetPer%20Mesh%20Transforms) (Math|Float|Truncate (.pscale (Utilities|Struct|BreakCSVPointFormat _returnvalue_8)))))) _location)) (Math|Rotator|CombineRotators (Class|KismetMathLibrary|QuatRotator (Class|KismetMathLibrary|MakeQuat (.Nx (Utilities|Struct|BreakCSVPointFormat _returnvalue_8)) (.Nz (Utilities|Struct|BreakCSVPointFormat _returnvalue_8)) (.Ny (Utilities|Struct|BreakCSVPointFormat _returnvalue_8)) (* (Math|Float|Sqrt (- (- (- (Math|Float|MakeLiteralFloat 1.0) (* (.Nx (Utilities|Struct|BreakCSVPointFormat _returnvalue_8)) (.Nx (Utilities|Struct|BreakCSVPointFormat _returnvalue_8)))) (* (.Ny (Utilities|Struct|BreakCSVPointFormat _returnvalue_8)) (.Ny (Utilities|Struct|BreakCSVPointFormat _returnvalue_8)))) (* (.Nz (Utilities|Struct|BreakCSVPointFormat _returnvalue_8)) (.Nz (Utilities|Struct|BreakCSVPointFormat _returnvalue_8))))) -1.0))) (Math|Rotator|CombineRotators (.Rotation (Math|Transform|BreakTransform (Utilities|Array|Get(acopy) (Variables|ExtraTransforms|GetPer%20Mesh%20Transforms) (Math|Float|Truncate (.pscale (Utilities|Struct|BreakCSVPointFormat _returnvalue_8)))))) _rotation)) (* (Math|Vector|MakeVector (.UVx (Utilities|Struct|BreakCSVPointFormat _returnvalue_8)) (.UVz (Utilities|Struct|BreakCSVPointFormat _returnvalue_8)) (.UVy (Utilities|Struct|BreakCSVPointFormat _returnvalue_8))) (* (.Scale (Math|Transform|BreakTransform (Utilities|Array|Get(acopy) (Variables|ExtraTransforms|GetPer%20Mesh%20Transforms) (Math|Float|Truncate (.pscale (Utilities|Struct|BreakCSVPointFormat _returnvalue_8)))))) _scale))) (.pscale (Utilities|Struct|BreakCSVPointFormat _returnvalue_9)) (Math|Vector4|MakeVector4 (.UVx (Utilities|Struct|BreakCSVPointFormat _returnvalue_9)) (.UVy (Utilities|Struct|BreakCSVPointFormat _returnvalue_9)) (.UVz (Utilities|Struct|BreakCSVPointFormat _returnvalue_9)) 1.0)) (LocalVariables|GetMetaData) "custom_float_2" (.UVz (Utilities|Struct|BreakCSVPointFormat _returnvalue_9)))
              (PCG|Metadata|SetFloatAttribute (Utilities|Struct|MakePCGPoint (Math|Transform|MakeTransform (+ (* (Math|Vector|MakeVector _expand_points _expand_points _expand_points) (Math|Vector|MakeVector (.Px (Utilities|Struct|BreakCSVPointFormat _returnvalue_8)) (.Pz (Utilities|Struct|BreakCSVPointFormat _returnvalue_8)) (.Py (Utilities|Struct|BreakCSVPointFormat _returnvalue_8)))) (+ (.Location (Math|Transform|BreakTransform (Utilities|Array|Get(acopy) (Variables|ExtraTransforms|GetPer%20Mesh%20Transforms) (Math|Float|Truncate (.pscale (Utilities|Struct|BreakCSVPointFormat _returnvalue_8)))))) _location)) (Math|Rotator|CombineRotators (Class|KismetMathLibrary|QuatRotator (Class|KismetMathLibrary|MakeQuat (.Nx (Utilities|Struct|BreakCSVPointFormat _returnvalue_8)) (.Nz (Utilities|Struct|BreakCSVPointFormat _returnvalue_8)) (.Ny (Utilities|Struct|BreakCSVPointFormat _returnvalue_8)) (* (Math|Float|Sqrt (- (- (- (Math|Float|MakeLiteralFloat 1.0) (* (.Nx (Utilities|Struct|BreakCSVPointFormat _returnvalue_8)) (.Nx (Utilities|Struct|BreakCSVPointFormat _returnvalue_8)))) (* (.Ny (Utilities|Struct|BreakCSVPointFormat _returnvalue_8)) (.Ny (Utilities|Struct|BreakCSVPointFormat _returnvalue_8)))) (* (.Nz (Utilities|Struct|BreakCSVPointFormat _returnvalue_8)) (.Nz (Utilities|Struct|BreakCSVPointFormat _returnvalue_8))))) -1.0))) (Math|Rotator|CombineRotators (.Rotation (Math|Transform|BreakTransform (Utilities|Array|Get(acopy) (Variables|ExtraTransforms|GetPer%20Mesh%20Transforms) (Math|Float|Truncate (.pscale (Utilities|Struct|BreakCSVPointFormat _returnvalue_8)))))) _rotation)) (* (Math|Vector|MakeVector (.UVx (Utilities|Struct|BreakCSVPointFormat _returnvalue_8)) (.UVz (Utilities|Struct|BreakCSVPointFormat _returnvalue_8)) (.UVy (Utilities|Struct|BreakCSVPointFormat _returnvalue_8))) (* (.Scale (Math|Transform|BreakTransform (Utilities|Array|Get(acopy) (Variables|ExtraTransforms|GetPer%20Mesh%20Transforms) (Math|Float|Truncate (.pscale (Utilities|Struct|BreakCSVPointFormat _returnvalue_8)))))) _scale))) (.pscale (Utilities|Struct|BreakCSVPointFormat _returnvalue_9)) (Math|Vector4|MakeVector4 (.UVx (Utilities|Struct|BreakCSVPointFormat _returnvalue_9)) (.UVy (Utilities|Struct|BreakCSVPointFormat _returnvalue_9)) (.UVz (Utilities|Struct|BreakCSVPointFormat _returnvalue_9)) 1.0)) (LocalVariables|GetMetaData) "custom_float_3" (.pscale (Utilities|Struct|BreakCSVPointFormat _returnvalue_9)))
              ;[1 1 1] Set Mesh Attribute
              (Class|PCGMetadataAccessorHelpers|SetStringAttribute (Utilities|Struct|MakePCGPoint (Math|Transform|MakeTransform (+ (* (Math|Vector|MakeVector _expand_points _expand_points _expand_points) (Math|Vector|MakeVector (.Px (Utilities|Struct|BreakCSVPointFormat _returnvalue_8)) (.Pz (Utilities|Struct|BreakCSVPointFormat _returnvalue_8)) (.Py (Utilities|Struct|BreakCSVPointFormat _returnvalue_8)))) (+ (.Location (Math|Transform|BreakTransform (Utilities|Array|Get(acopy) (Variables|ExtraTransforms|GetPer%20Mesh%20Transforms) (Math|Float|Truncate (.pscale (Utilities|Struct|BreakCSVPointFormat _returnvalue_8)))))) _location)) (Math|Rotator|CombineRotators (Class|KismetMathLibrary|QuatRotator (Class|KismetMathLibrary|MakeQuat (.Nx (Utilities|Struct|BreakCSVPointFormat _returnvalue_8)) (.Nz (Utilities|Struct|BreakCSVPointFormat _returnvalue_8)) (.Ny (Utilities|Struct|BreakCSVPointFormat _returnvalue_8)) (* (Math|Float|Sqrt (- (- (- (Math|Float|MakeLiteralFloat 1.0) (* (.Nx (Utilities|Struct|BreakCSVPointFormat _returnvalue_8)) (.Nx (Utilities|Struct|BreakCSVPointFormat _returnvalue_8)))) (* (.Ny (Utilities|Struct|BreakCSVPointFormat _returnvalue_8)) (.Ny (Utilities|Struct|BreakCSVPointFormat _returnvalue_8)))) (* (.Nz (Utilities|Struct|BreakCSVPointFormat _returnvalue_8)) (.Nz (Utilities|Struct|BreakCSVPointFormat _returnvalue_8))))) -1.0))) (Math|Rotator|CombineRotators (.Rotation (Math|Transform|BreakTransform (Utilities|Array|Get(acopy) (Variables|ExtraTransforms|GetPer%20Mesh%20Transforms) (Math|Float|Truncate (.pscale (Utilities|Struct|BreakCSVPointFormat _returnvalue_8)))))) _rotation)) (* (Math|Vector|MakeVector (.UVx (Utilities|Struct|BreakCSVPointFormat _returnvalue_8)) (.UVz (Utilities|Struct|BreakCSVPointFormat _returnvalue_8)) (.UVy (Utilities|Struct|BreakCSVPointFormat _returnvalue_8))) (* (.Scale (Math|Transform|BreakTransform (Utilities|Array|Get(acopy) (Variables|ExtraTransforms|GetPer%20Mesh%20Transforms) (Math|Float|Truncate (.pscale (Utilities|Struct|BreakCSVPointFormat _returnvalue_8)))))) _scale))) (.pscale (Utilities|Struct|BreakCSVPointFormat _returnvalue_9)) (Math|Vector4|MakeVector4 (.UVx (Utilities|Struct|BreakCSVPointFormat _returnvalue_9)) (.UVy (Utilities|Struct|BreakCSVPointFormat _returnvalue_9)) (.UVz (Utilities|Struct|BreakCSVPointFormat _returnvalue_9)) 1.0)) (LocalVariables|GetMetaData) "mesh" (Utilities|Array|Get(acopy) _returnvalue (Math|Float|Truncate (.pscale (Utilities|Struct|BreakCSVPointFormat _returnvalue_8)))))))
          (return (Utilities|Struct|MakePCGPoint (Math|Transform|MakeTransform (+ (* (Math|Vector|MakeVector _expand_points _expand_points _expand_points) (Math|Vector|MakeVector (.Px (Utilities|Struct|BreakCSVPointFormat _returnvalue_8)) (.Pz (Utilities|Struct|BreakCSVPointFormat _returnvalue_8)) (.Py (Utilities|Struct|BreakCSVPointFormat _returnvalue_8)))) (+ (.Location (Math|Transform|BreakTransform (Utilities|Array|Get(acopy) (Variables|ExtraTransforms|GetPer%20Mesh%20Transforms) (Math|Float|Truncate (.pscale (Utilities|Struct|BreakCSVPointFormat _returnvalue_8)))))) _location)) (Math|Rotator|CombineRotators (Class|KismetMathLibrary|QuatRotator (Class|KismetMathLibrary|MakeQuat (.Nx (Utilities|Struct|BreakCSVPointFormat _returnvalue_8)) (.Nz (Utilities|Struct|BreakCSVPointFormat _returnvalue_8)) (.Ny (Utilities|Struct|BreakCSVPointFormat _returnvalue_8)) (* (Math|Float|Sqrt (- (- (- (Math|Float|MakeLiteralFloat 1.0) (* (.Nx (Utilities|Struct|BreakCSVPointFormat _returnvalue_8)) (.Nx (Utilities|Struct|BreakCSVPointFormat _returnvalue_8)))) (* (.Ny (Utilities|Struct|BreakCSVPointFormat _returnvalue_8)) (.Ny (Utilities|Struct|BreakCSVPointFormat _returnvalue_8)))) (* (.Nz (Utilities|Struct|BreakCSVPointFormat _returnvalue_8)) (.Nz (Utilities|Struct|BreakCSVPointFormat _returnvalue_8))))) -1.0))) (Math|Rotator|CombineRotators (.Rotation (Math|Transform|BreakTransform (Utilities|Array|Get(acopy) (Variables|ExtraTransforms|GetPer%20Mesh%20Transforms) (Math|Float|Truncate (.pscale (Utilities|Struct|BreakCSVPointFormat _returnvalue_8)))))) _rotation)) (* (Math|Vector|MakeVector (.UVx (Utilities|Struct|BreakCSVPointFormat _returnvalue_8)) (.UVz (Utilities|Struct|BreakCSVPointFormat _returnvalue_8)) (.UVy (Utilities|Struct|BreakCSVPointFormat _returnvalue_8))) (* (.Scale (Math|Transform|BreakTransform (Utilities|Array|Get(acopy) (Variables|ExtraTransforms|GetPer%20Mesh%20Transforms) (Math|Float|Truncate (.pscale (Utilities|Struct|BreakCSVPointFormat _returnvalue_8)))))) _scale))) (.pscale (Utilities|Struct|BreakCSVPointFormat _returnvalue_9)) (Math|Vector4|MakeVector4 (.UVx (Utilities|Struct|BreakCSVPointFormat _returnvalue_9)) (.UVy (Utilities|Struct|BreakCSVPointFormat _returnvalue_9)) (.UVz (Utilities|Struct|BreakCSVPointFormat _returnvalue_9)) 1.0)) true))))))